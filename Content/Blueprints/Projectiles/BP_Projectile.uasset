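; Base-style projectile actor that pops enemies, loses one Pierce per hit, and destroys itself when Pierce runs out or its Lifetime ends.
; On BeginPlay it generates a random ProjectileTag, which the tag-test function and macro write into an enemy's ImuneTags to tell new touches from repeat ones.
; Collision detection and movement are absent from these graphs; OnHitEnemy only applies Pop and damage types to the enemy it receives.
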(event Custom|OnHitEnemy
  (params (Enemy :type BP%20Enemy%20Object%20Reference))
  (Utilities|IsValid Enemy
    (:Is%20Valid
      (Default|Pop Enemy (Variables|Default|GetPop) (Variables|Default|GetDamageTypes))
      (Math|Integer|DecrementInt (Variables|Default|GetPierce)
        (:%20%20
          (if (<= (Variables|Default|GetPierce) 0)
            (Actor|DestroyActor)))))))

(event EventBeginPlay
  (Variables|Default|SetProjectileTag (CallFunction|RandomHash 20))
  (Utilities|FlowControl|Delay (Variables|Default|GetLifetime))
  (Actor|DestroyActor))

(event Collision|EventActorBeginOverlap
  (params (OtherActor :type Actor%20Object%20Reference)))

(event EventTick
  (params (DeltaSeconds :type Float%20%28single-precision%29)))

(fn ConstructionScript)

(fn IsEnemyTagged
  (params (Enemy :type BP%20Enemy%20Object%20Reference))
  (return (Utilities|Set|Contains (Variables|/Game/Blueprints/Enemies/BP_Enemy.BP_Enemy_C|GetImuneTags Enemy) (Variables|Default|GetProjectileTag))))

(fn EnemyTagTestFunction
  (params (Object :type Object%20Object%20Reference))
  (bind _asbp_enemy (Utilities|Casting|CastToBP_Enemy Object))
  (bind _output_get (LocalVariables|SetEnemyWasTagged (CallFunction|IsEnemyTagged _asbp_enemy)))
  (if _output_get
    _
    (else
      (Utilities|Set|Add (Variables|/Game/Blueprints/Enemies/BP_Enemy.BP_Enemy_C|GetImuneTags _asbp_enemy) (Variables|Default|GetProjectileTag))))
  (return (not (LocalVariables|GetEnemyWasTagged)) _asbp_enemy))