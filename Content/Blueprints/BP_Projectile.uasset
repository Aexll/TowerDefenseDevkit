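; BP_Projectile is a projectile that pops BP_Enemy actors it overlaps and can pierce several before it is destroyed.
; It moves forward along its root component every tick by Speed, without sweeping.
; A random tag made at BeginPlay is added to each enemy's immune list, so one projectile hits each enemy only once.
; Each new hit calls the enemy's Pop with the projectile's Pop value and decrements Pierce, destroying the actor at zero.
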(event OnComponentBeginOverlap(Capsule)
  (params (OverlappedComponent :type Primitive%20Component%20Object%20Reference) (OtherActor :type Actor%20Object%20Reference) (OtherComp :type Primitive%20Component%20Object%20Reference) (OtherBodyIndex :type Integer) (bFromSweep :type Boolean) (SweepResult :type Hit%20Result%20Structure%20%28by%20ref%29))
  (bind _projectiletag (Variables|Default|GetProjectileTag))
  (bind _asbp_enemy (Utilities|Casting|CastToBP_Enemy OtherActor))
  (if (not (Utilities|Set|Contains (Variables|/Game/Blueprints/BP_Enemy.BP_Enemy_C|GetImuneTags _asbp_enemy) _projectiletag))
    (Utilities|Set|Add (Variables|/Game/Blueprints/BP_Enemy.BP_Enemy_C|GetImuneTags _asbp_enemy) _projectiletag)
    (Default|Pop _asbp_enemy (Variables|Default|GetPop))
    (Math|Integer|DecrementInt (Variables|Default|GetPierce)
      (:%20%20
        (if (<= (Variables|Default|GetPierce) 0)
          (Actor|DestroyActor))))))

(event EventBeginPlay
  (Variables|Default|SetProjectileTag (CallFunction|RandomHash 20)))

(event Collision|EventActorBeginOverlap
  (params (OtherActor :type Actor%20Object%20Reference)))

(event EventTick
  (params (DeltaSeconds :type Float%20%28single-precision%29))
  (Transformation|AddActorWorldOffset (* DeltaSeconds (Math|Vector|GetForwardVector (Variables|Default|GetDefaultSceneRoot)) (Variables|Default|GetSpeed) 1e+02)))

(fn ConstructionScript)