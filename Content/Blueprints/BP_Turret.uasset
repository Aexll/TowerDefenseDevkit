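; BP_Turret is a turret that automatically aims and fires at BP_Enemy actors.
; Each Tick it gathers all enemies and rotates Cube1 to face the first one in the array, with no distance or range check.
; A Delay of one over AttackSpeed within Tick paces the fire, after which a Projectile spawns at the Arrow component's transform.
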(event EventBeginPlay)

(event Collision|EventActorBeginOverlap
  (params (OtherActor :type Actor%20Object%20Reference)))

(event EventTick
  (params (DeltaSeconds :type Float%20%28single-precision%29))
  (bind _outactors (Actor|GetAllActorsOfClass "/Game/Blueprints/BP_Enemy.BP_Enemy_C"))
  (if (Utilities|Array|IsValidIndex _outactors)
    (Transformation|SetWorldRotation (Variables|Default|GetCube1) (Math|Rotator|FindLookatRotation (Transformation|GetWorldLocation (Variables|Default|GetCube1)) (Transformation|GetActorLocation (Utilities|Array|Get(acopy) _outactors))) false false)
    (Utilities|FlowControl|Delay (/ 1.0 (Variables|Default|GetAttackSpeed)))
    (Game|SpawnActorfromClass (Variables|Default|GetProjectile) (Transformation|GetWorldTransform (Variables|Default|GetArrow)) "Undefined" 0 0)))

(fn ConstructionScript)