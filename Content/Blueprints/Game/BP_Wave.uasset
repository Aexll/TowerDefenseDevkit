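; BP_Wave is a wave spawner actor that releases one configured wave of enemies and then destroys itself.
; On BeginPlay it waits for the wave's start time, then starts a looping timer at the wave's frequency.
; Each tick of the timer looks up the unit's row in the CoreUnits data table and spawns a BP_Enemy, passing it the path, row data and modifiers, until the amount runs out.
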(event Custom|SpawnUnit
  (bind _wave (Variables|Default|GetWave))
  (bind (_unit _modifiers) (Utilities|Struct|BreakS_Unit (.unit _wave)))
  (if (> (Variables|Default|GetSpawnLeft) 0)
    (Math|Integer|DecrementInt (Variables|Default|GetSpawnLeft)
      (:%20%20
        (bind _returnvalue (Utilities|GetDataTableRow "/Game/Blueprints/Datas/CoreUnits.CoreUnits" _unit)
          (:then
            (Game|SpawnActorfromClass "/Game/Blueprints/Enemies/BP_Enemy.BP_Enemy_C" (Math|Transform|MakeTransform "0, 0, 0") "Undefined" 0 (Variables|Default|GetPath) 0.0 _returnvalue _modifiers 0 0)))))
    (else
      (Actor|DestroyActor))))

(event EventBeginPlay
  (bind _wave (Variables|Default|GetWave))
  (Utilities|FlowControl|Delay (.time _wave))
  (Variables|Default|SetSpawnLeft (.amount _wave))
  (Utilities|Time|SetTimerbyEvent (delegate Custom|SpawnUnit) (.frequency _wave) true))

(event Collision|EventActorBeginOverlap
  (params (OtherActor :type Actor%20Object%20Reference)))

(event EventTick
  (params (DeltaSeconds :type Float%20%28single-precision%29)))

(fn ConstructionScript)