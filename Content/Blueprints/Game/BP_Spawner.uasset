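; BP_Spawner launches enemy rounds by spawning a BP_Wave actor for each wave in the selected round, passing it the spawner's path.
; GetMaxTime derives round length from the latest wave end: start time plus amount times frequency.
; Tick counts that time down and writes the remaining fraction to GM_Game's RoundPercent.
; An unconnected delayed loop that spawns BP_Enemy from CoreUnits data table rows never runs.
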(event Custom|LaunchRound
  (params (Round :type Integer))
  (bind _maxtime1 (CallFunction|GetMaxTime Round))
  (bind _output_get (Variables|Default|SetTimeLeft _maxtime1))
  (Variables|Default|SetRoundMaxTime _output_get)
  (for _array_element (Utilities|Struct|BreakS_Round (Utilities|Array|Get(acopy) (Variables|Default|GetRound) Round))
    (Game|SpawnActorfromClass "/Game/Blueprints/Game/BP_Wave.BP_Wave_C" (Math|Transform|MakeTransform "0, 0, 0") "Undefined" 0 _array_element (Variables|Default|GetPath) 0)))

(event EventBeginPlay
  (bind _asgm_game (Utilities|Casting|CastToGM_Game (Game|GetGameMode)))
  (Variables|Default|SetGM _asgm_game))

(event Collision|EventActorBeginOverlap
  (params (OtherActor :type Actor%20Object%20Reference)))

(event EventTick
  (params (DeltaSeconds :type Float%20%28single-precision%29))
  (bind _output_get (Variables|Default|SetTimeLeft (- (Variables|Default|GetTimeLeft) DeltaSeconds)))
  (Variables|/Game/Blueprints/Game/GM_Game.GM_Game_C|SetRoundPercent (Variables|Default|GetGM) (/ _output_get (Variables|Default|GetRoundMaxTime))))

(fn ConstructionScript)

(fn GetMaxTime
  (params (Round :type Integer))
  (for _array_element (Utilities|Struct|BreakS_Round (Utilities|Array|Get(acopy) (Variables|Default|GetRound) Round))
    (if (> (+ (.Time (Utilities|Struct|BreakS_Wave _array_element)) (* (.Amount (Utilities|Struct|BreakS_Wave _array_element)) (.Frequency (Utilities|Struct|BreakS_Wave _array_element)))) (LocalVariables|GetMaxTime))
      (LocalVariables|SetMaxTime (+ (.Time (Utilities|Struct|BreakS_Wave _array_element)) (* (.Amount (Utilities|Struct|BreakS_Wave _array_element)) (.Frequency (Utilities|Struct|BreakS_Wave _array_element)))))))
  (return (LocalVariables|GetMaxTime)))