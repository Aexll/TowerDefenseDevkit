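; GM_Game is the game mode that relays round starts to spawners and tracks the health that decides a loss.
; On BeginPlay it binds to the LaunchRound event, then forwards each round number to every BP_Spawner in the level.
; TakeDamages subtracts from Health and, at zero or below, calls OnGameLost, which adds the lose widget to the first player's viewport.
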(event Custom|TakeDamages
  (params (Amount :type Integer))
  (bind _output_get (Variables|Default|SetHealth (- (Variables|Default|GetHealth) Amount)))
  (if (<= _output_get 0)
    (CallFunction|OnGameLost)))

(event Custom|OnGameLost
  (bind _returnvalue (UserInterface|CreateWidget "/Game/Widgets/WIdget_Lose.WIdget_Lose_C" (Game|GetPlayerController 0)))
  (UserInterface|Viewport|AddtoViewport _returnvalue 0))

(event Custom|LaunchRound_Event
  (params (Number :type Integer))
  (bind _outactors (Actor|GetAllActorsOfClass "/Game/Blueprints/Game/BP_Spawner.BP_Spawner_C"))
  (for _array_element _outactors
    (Default|LaunchRound _array_element Number)))

(event EventBeginPlay
  (EventDispatchers|BindEventtoLaunchRound (delegate Custom|LaunchRound_Event)))

(event EventTick
  (params (DeltaSeconds :type Float%20%28single-precision%29)))

(fn ConstructionScript)