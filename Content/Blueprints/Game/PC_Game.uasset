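; Player controller for turret placement and selection in a tower-defense game, which also creates the main HUD.
; Tick moves a preview actor to the traced surface point, aligns it to the normal and flags validity via an overlap sphere trace.
; Left click selects a turret or attempts to buy and spawn the previewed one, right click cancels, and P launches the round.
; A shared helper traces from either the cursor or camera center.
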(event Custom|SelectTower_Event
  (params (SelectedTower :type BP%20Turret%20Object%20Reference))
  (Variables|Default|SetSelectedTurret SelectedTower))

(event Custom|SpawnTurretAtPosition
  (params (Turret :type BP%20Turret%20Class%20Reference) (Position :type Vector))
  ;[0 0 0] Spawn turret at position
  (bind _bought (CallFunction|TryBuy (Utilities|GetClassDefaults Turret)))
  (if _bought
    (Game|SpawnActorfromClass Turret (Math|Transform|MakeTransform Position) "Undefined" 0 0))
  (Variables|Default|SetPreviewTurret 0))

(event EventBeginPlay
  (bind _returnvalue (UserInterface|CreateWidget "/Game/Widgets/HUD_MainGame.HUD_MainGame_C"))
  (bind _output_get (Variables|Default|SetMainGameWidget _returnvalue))
  (UserInterface|Viewport|AddtoViewport _output_get 0)
  (EventDispatchers|BindEventtoSelectTower (delegate Custom|SelectTower_Event))
  ;[0 0 0] Spawn the preview instance
  (bind _returnvalue_2 (Game|SpawnActorfromClass "/Game/Blueprints/Turrets/BP_TurretPreview.BP_TurretPreview_C" (Math|Transform|MakeTransform "0, 0, 0") "Undefined" 0 0))
  (bind _output_get_2 (Variables|Default|SetPreviewInstance _returnvalue_2))
  (Default|SetVisibility _output_get_2 false))

(event EventTick
  (params (DeltaSeconds :type Float%20%28single-precision%29))
  (bind _previewinstance (Variables|Default|GetPreviewInstance))
  (bind _previewinstance_2 (Variables|Default|GetPreviewInstance))
  (bind _previewturret (Variables|Default|GetPreviewTurret))
  ;[0 0 0] Tick
  (bind (_outhit _returnvalue) (CallFunction|MouseClickonScene "TraceTypeQuery1"))
  (if _returnvalue
    (if (Utilities|IsValidClass _previewturret)
      (Default|SetVisibility _previewinstance_2 true)
      (bind _outhit_2 (Collision|SphereTraceByChannel (.Location (Collision|BreakHitResult _outhit)) (.Location (Collision|BreakHitResult _outhit)) (Utilities|GetClassDefaults _previewturret) "TraceTypeQuery3" false 0 "None"))
      (Transformation|SetActorLocation _previewinstance (.Location (Collision|BreakHitResult _outhit)) false false)
      (Default|SetValidity _previewinstance (not (.bBlockingHit (Collision|BreakHitResult _outhit_2))))
      (Transformation|SetActorRotation _previewinstance (Math|Rotator|MakeRotfromZ (.ImpactNormal (Collision|BreakHitResult _outhit))))
      (else
        (Default|SetVisibility _previewinstance_2 false)))))

(event Input|MouseEvents|LeftMouseButton
  (params (Key :type Key%20Structure :default "None")))

(event Input|MouseEvents|LeftMouseButton
  (params (Key :type Key%20Structure :default "None"))
  (bind _previewturret (Variables|Default|GetPreviewTurret))
  ;[0 0 0] OnClick
  (:Pressed
    (bind (_outhit _returnvalue) (CallFunction|MouseClickonScene "TraceTypeQuery3"))
    (if _returnvalue
      (bind _asbp_turret (Utilities|Casting|CastToBP_Turret (.HitActor (Collision|BreakHitResult _outhit))))
      (Default|Select _asbp_turret)
      (else
        (bind (_outhit_2 _returnvalue_2) (CallFunction|MouseClickonScene "TraceTypeQuery1"))
        (if _returnvalue_2
          (if (Utilities|IsValidClass _previewturret)
            (bind _returnvalue_3 (Collision|SphereTraceByChannel (.Location (Collision|BreakHitResult _outhit_2)) (.Location (Collision|BreakHitResult _outhit_2)) (Utilities|GetClassDefaults _previewturret) "TraceTypeQuery3" false 0 "None"))
            (if (not _returnvalue_3)
              (CallFunction|SpawnTurretatPosition (Variables|Default|GetPreviewTurret) (.Location (Collision|BreakHitResult _outhit_2)))
              (Default|CallSelectTower))))))))

(event Input|MouseEvents|RightMouseButton
  (params (Key :type Key%20Structure :default "None"))
  (:Pressed
    (Variables|Default|SetPreviewTurret 0)))

(event Input|KeyboardEvents|P
  (params (Key :type Key%20Structure :default "None"))
  (:Pressed
    (bind _asgm_game (Utilities|Casting|CastToGM_Game (Game|GetGameMode)))
    (Default|LaunchRoundEvent _asgm_game (Variables|/Game/Blueprints/Game/GM_Game.GM_Game_C|GetRound _asgm_game))))

(fn ConstructionScript)

(fn MouseClickonScene
  (params (TraceChannel :type ETraceTypeQuery%20Enum :default "TraceTypeQuery1"))
  (bind _returnvalue (Game|GetPlayerController 0))
  (bind _playercameramanager (Variables|Default|GetPlayerCameraManager))
  (bind _tracefromcamera (Variables|Default|GetTraceFromCamera))
  (bind _returnvalue_2 (Camera|GetCameraLocation _playercameramanager))
  (bind (_worldlocation _worlddirection) (Game|Player|ConvertMouseLocationToWorldSpace _returnvalue))
  (bind (_outhit _returnvalue_3) (Collision|LineTraceByChannel (Math|Vector|SelectVector _returnvalue_2 _worldlocation _tracefromcamera) (Math|Vector|SelectVector (+ _returnvalue_2 (* (Math|Vector|GetForwardVector (Camera|GetCameraRotation _playercameramanager)) 10000)) (+ _worldlocation (* _worlddirection 10000)) _tracefromcamera) TraceChannel false 0 "None"))
  (return _outhit _returnvalue_3))