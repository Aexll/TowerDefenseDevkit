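; BP_FPSView is the first-person player pawn, handling look and movement input and toggling between camera aiming and a cursor-driven tower HUD mode.
; E drives a FlipFlop that switches PC_Game's cursor, camera tracing and input mode, and shows or hides the tower and turret shop widgets.
; BeginPlay caches the controller and fires the FlipFlop twice, so play starts in game-only mode with those widgets hidden.
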(event EventBeginPlay
  (bind _aspc_game (Utilities|Casting|CastToPC_Game (Game|GetPlayerController 0)))
  (bind _output_get (Variables|Default|SetPCGame _aspc_game))
  (Variables|/Script/Engine.PlayerController|SetbShowMouseCursor _output_get false)
  (Variables|/Game/Blueprints/Game/PC_Game.PC_Game_C|SetTraceFromCamera _output_get true)
  (Utilities|FlowControl|Sequence
    (:then_0
      _)
    (:then_1
      _))
  (Utilities|FlowControl|FlipFlop
    (:A
      (Variables|/Script/Engine.PlayerController|SetbShowMouseCursor (Variables|Default|GetPCGame) true)
      (Variables|/Game/Blueprints/Game/PC_Game.PC_Game_C|SetTraceFromCamera (Variables|Default|GetPCGame) false)
      (Input|SetInputModeGameandUI (Variables|Default|GetPCGame) 0 "DoNotLock" true)
      (Widget|SetVisibility (Variables|/Game/Widgets/HUD_MainGame.HUD_MainGame_C|GetHUD_Tower (Variables|/Game/Blueprints/Game/PC_Game.PC_Game_C|GetMainGameWidget (Variables|Default|GetPCGame))) "Visible"))
    (:B
      (Variables|/Script/Engine.PlayerController|SetbShowMouseCursor (Variables|Default|GetPCGame) false)
      (Variables|/Game/Blueprints/Game/PC_Game.PC_Game_C|SetTraceFromCamera (Variables|Default|GetPCGame) true)
      (Input|SetInputModeGameOnly (Variables|Default|GetPCGame))
      (Widget|SetVisibility (Variables|/Game/Widgets/HUD_MainGame.HUD_MainGame_C|GetHUD_Tower (Variables|/Game/Blueprints/Game/PC_Game.PC_Game_C|GetMainGameWidget (Variables|Default|GetPCGame))) "Hidden"))))

(event Collision|EventActorBeginOverlap
  (params (OtherActor :type Actor%20Object%20Reference)))

(event EventTick
  (params (DeltaSeconds :type Float%20%28single-precision%29)))

(event Input|AxisEvents|InputAxisLookUp
  (params (AxisValue :type Float%20%28single-precision%29))
  (Pawn|Input|AddControllerPitchInput AxisValue))

(event Input|AxisEvents|InputAxisLookRight
  (params (AxisValue :type Float%20%28single-precision%29))
  (Pawn|Input|AddControllerYawInput AxisValue))

(event Input|AxisEvents|InputAxisMoveForward
  (params (AxisValue :type Float%20%28single-precision%29))
  (Pawn|Input|AddMovementInput (Math|Vector|GetForwardVector (Variables|Collision|GetCapsuleComponent)) AxisValue false))

(event Input|AxisEvents|InputAxisMoveRight
  (params (AxisValue :type Float%20%28single-precision%29))
  (Pawn|Input|AddMovementInput (Math|Vector|GetRightVector (Variables|Collision|GetCapsuleComponent)) AxisValue false))

(event Input|KeyboardEvents|E
  (params (Key :type Key%20Structure :default "None"))
  (bind _pcgame (Variables|Default|GetPCGame))
  (bind _pcgame_2 (Variables|Default|GetPCGame))
  (bind _pcgame_3 (Variables|Default|GetPCGame))
  (bind _maingamewidget (Variables|/Game/Blueprints/Game/PC_Game.PC_Game_C|GetMainGameWidget _pcgame_2))
  (bind _hud_tower (Variables|/Game/Widgets/HUD_MainGame.HUD_MainGame_C|GetHUD_Tower _maingamewidget))
  (:Pressed
    (Utilities|FlowControl|FlipFlop
      (:A
        (Variables|/Script/Engine.PlayerController|SetbShowMouseCursor _pcgame true)
        (Variables|/Game/Blueprints/Game/PC_Game.PC_Game_C|SetTraceFromCamera _pcgame false)
        (Input|SetInputModeGameandUI _pcgame_3 0 "DoNotLock" true)
        (Widget|SetVisibility _hud_tower "Visible"))
      (:B
        (Variables|/Script/Engine.PlayerController|SetbShowMouseCursor _pcgame false)
        (Variables|/Game/Blueprints/Game/PC_Game.PC_Game_C|SetTraceFromCamera _pcgame true)
        (Input|SetInputModeGameOnly _pcgame_3)
        (Widget|SetVisibility _hud_tower "Hidden")))))

(fn ConstructionScript)