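; BP_Base is the base actor that costs the player health when an enemy reaches it.
; Its Box overlap filters for BP_Enemy and fires the OnEnemyCollide dispatcher, which the actor binds to itself at BeginPlay.
; While GM_Game health is at least zero, the handler applies the enemy's calculated money drop as damage to the game mode and destroys the enemy.
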(event OnComponentBeginOverlap(Box)
  (params (OverlappedComponent :type Primitive%20Component%20Object%20Reference) (OtherActor :type Actor%20Object%20Reference) (OtherComp :type Primitive%20Component%20Object%20Reference) (OtherBodyIndex :type Integer) (bFromSweep :type Boolean) (SweepResult :type Hit%20Result%20Structure%20%28by%20ref%29))
  (bind _asbp_enemy (Utilities|Casting|CastToBP_Enemy OtherActor))
  (Default|CallOnEnemyCollide _asbp_enemy))

(event Custom|OnEnemyCollide_Event
  (params (Target :type BP%20Enemy%20Object%20Reference))
  (bind _gm (Variables|Default|GetGM))
  (bind _moneydroped (Default|CalculateDrops Target 100))
  (if (>= (Variables|/Game/Blueprints/Game/GM_Game.GM_Game_C|GetHealth _gm) 0)
    (Default|TakeDamages _gm _moneydroped)
    (Actor|DestroyActor Target)))

(event EventBeginPlay
  (bind _asgm_game (Utilities|Casting|CastToGM_Game (Game|GetGameMode)))
  (Variables|Default|SetGM _asgm_game)
  (EventDispatchers|BindEventtoOnEnemyCollide (delegate Custom|OnEnemyCollide_Event)))

(event Collision|EventActorBeginOverlap
  (params (OtherActor :type Actor%20Object%20Reference)))

(event EventTick
  (params (DeltaSeconds :type Float%20%28single-precision%29)))

(fn ConstructionScript)