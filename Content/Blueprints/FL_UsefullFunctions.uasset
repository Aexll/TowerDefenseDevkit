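; Blueprint function library of shared gameplay helpers for random strings, actor targeting and money.
; RandomHash builds strings from a random alphabet, and GetClosestActor scans by squared distance, returning the nearest actor and its distance.
; FocusEnemy selects a detected BP_Enemy by First or Last mode, comparing Time values against the first entry's, which is never updated.
; CanBuy, TryBuy and GainMoney check, spend and add Money on GM_Game.
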(fn RandomHash
  (params (Length :type Integer))
  (LocalVariables|SetRandomString "")
  (for _index (range 0 Length)
    (LocalVariables|SetRandomString (Utilities|String|Append (LocalVariables|GetRandomString) (.OutItem (Utilities|Array|Random (LocalVariables|GetAlphabet))))))
  (return (LocalVariables|GetRandomString)))

(fn GetClosestActor
  (params (Location :type Vector) (Actors :type Array%20of%20Actor%20Object%20References))
  (bind _output (Utilities|Array|Get(acopy) Actors))
  (if (Utilities|Array|IsValidIndex Actors)
    (LocalVariables|SetClosestActor _output)
    (LocalVariables|SetMinSquaredDistance (Class|KismetMathLibrary|VectorDistanceSquared Location (Transformation|GetActorLocation _output)))
    (for _array_element Actors
      (if (< (Class|KismetMathLibrary|VectorDistanceSquared Location (Transformation|GetActorLocation _array_element)) (LocalVariables|GetMinSquaredDistance))
        (LocalVariables|SetMinSquaredDistance (Class|KismetMathLibrary|VectorDistanceSquared Location (Transformation|GetActorLocation _array_element)))
        (LocalVariables|SetClosestActor _array_element)))
    (return (Math|Float|Sqrt (LocalVariables|GetMinSquaredDistance)) (LocalVariables|GetClosestActor))
    (else
      (return 0.0 0))))

(fn FocusEnemy
  (params (EnemysDetected :type Array%20of%20Actor%20Object%20References) (FocusType :type EFocus%20Enum :default "NewEnumerator0"))
  (if (not (Utilities|Enum|Equal(Enum) FocusType "NewEnumerator5"))
    (Utilities|FlowControl|Sequence
      (:then_0
        (bind _asbp_enemy (Utilities|Casting|CastToBP_Enemy (Utilities|Array|Get(acopy) EnemysDetected)))
        (bind _output_get (LocalVariables|SetSelectedEnemy _asbp_enemy))
        (switch Utilities|FlowControl|Switch|SwitchonEFocus FocusType
          (:NewEnumerator0
            (LocalVariables|SetSelectedEnemyDistance (Variables|/Game/Blueprints/Enemies/BP_Enemy.BP_Enemy_C|GetTime _output_get)))
          (:NewEnumerator1
            (LocalVariables|SetSelectedEnemyDistance (Variables|/Game/Blueprints/Enemies/BP_Enemy.BP_Enemy_C|GetTime _output_get)))))
      (:then_1
        (for _array_element EnemysDetected
          (bind _asbp_enemy_2 (Utilities|Casting|CastToBP_Enemy _array_element))
          (switch Utilities|FlowControl|Switch|SwitchonEFocus FocusType
            (:NewEnumerator0
              (if (> (Variables|/Game/Blueprints/Enemies/BP_Enemy.BP_Enemy_C|GetTime _asbp_enemy_2) (LocalVariables|GetSelectedEnemyDistance))
                (LocalVariables|SetSelectedEnemyDistance (LocalVariables|GetSelectedEnemyDistance))
                (LocalVariables|SetSelectedEnemy _asbp_enemy_2)))
            (:NewEnumerator1
              (if (< (Variables|/Game/Blueprints/Enemies/BP_Enemy.BP_Enemy_C|GetTime _asbp_enemy_2) (LocalVariables|GetSelectedEnemyDistance))
                (LocalVariables|SetSelectedEnemyDistance (LocalVariables|GetSelectedEnemyDistance))
                (LocalVariables|SetSelectedEnemy _asbp_enemy_2)))))
        (return (LocalVariables|GetSelectedEnemy) (LocalVariables|GetSelectedEnemyDistance))))
    (else
      (return 0 0.0))))

(fn CanBuy
  (params (Price :type Integer))
  (bind _asgm_game (Utilities|Casting|CastToGM_Game (Game|GetGameMode)))
  (return (>= (Variables|/Game/Blueprints/Game/GM_Game.GM_Game_C|GetMoney _asgm_game) Price)))

(fn TryBuy
  (params (Price :type Integer) (__WorldContext :type Object%20Object%20Reference))
  (bind _asgm_game (Utilities|Casting|CastToGM_Game (Game|GetGameMode)))
  (if (>= (Variables|/Game/Blueprints/Game/GM_Game.GM_Game_C|GetMoney _asgm_game) Price)
    (bind _output_get (Variables|/Game/Blueprints/Game/GM_Game.GM_Game_C|SetMoney _asgm_game (- (Variables|/Game/Blueprints/Game/GM_Game.GM_Game_C|GetMoney _asgm_game) Price)))
    (return true _output_get)
    (else
      (return false (Variables|/Game/Blueprints/Game/GM_Game.GM_Game_C|GetMoney _asgm_game)))))

(fn GainMoney
  (params (Amount :type Integer))
  (bind _asgm_game (Utilities|Casting|CastToGM_Game (Game|GetGameMode)))
  (Variables|/Game/Blueprints/Game/GM_Game.GM_Game_C|SetMoney _asgm_game (+ (Variables|/Game/Blueprints/Game/GM_Game.GM_Game_C|GetMoney _asgm_game) Amount)))