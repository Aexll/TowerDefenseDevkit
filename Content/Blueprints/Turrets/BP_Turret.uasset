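; BP_Turret is a placeable turret that the player can select and upgrade, with no targeting or firing logic in this graph.
; Select toggles it as the PC_Game controller's selected turret and clears any preview turret, while Tick shows the range viewer only while selected.
; Upgrading spawns the given class at its transform, fires AfterUpgrade with the new actor, then destroys itself.
; The construction script sizes range and blocking volumes from Range and Size.
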(event Custom|Select
  (bind _self self)
  (bind _pc (Variables|Default|GetPC))
  ;[1 0.1042 0.6348] OnSelected
  (Default|CallSelectTower _pc (select (== (Variables|/Game/Blueprints/Game/PC_Game.PC_Game_C|GetSelectedTurret _pc) _self) 0 _self))
  (Variables|/Game/Blueprints/Game/PC_Game.PC_Game_C|SetPreviewTurret (Variables|Default|GetPC) 0))

(event Custom|Upgrade_Event
  (params (NewParam :type BP%20Turret%20Class%20Reference))
  ;[1 0.03955 0.03955] Bind Upgrade
  (bind _returnvalue (Game|SpawnActorfromClass NewParam (Transformation|GetActorTransform self) "Undefined" 0 0))
  (Default|CallAfterUpgrade _returnvalue)
  (Actor|DestroyActor))

(event EventBeginPlay
  ;[1 0.03955 0.03955] Bind Upgrade
  (EventDispatchers|BindEventtoUpgrade (delegate Custom|Upgrade_Event))
  ;[0 0.4599 1] Definitions
  (bind _aspc_game (Utilities|Casting|CastToPC_Game (Game|GetPlayerController 0)))
  (Variables|Default|SetPC _aspc_game))

(event Collision|EventActorBeginOverlap
  (params (OtherActor :type Actor%20Object%20Reference)))

(event EventTick
  (params (DeltaSeconds :type Float%20%28single-precision%29))
  ;[0 0 0] Show or hide the range viewer
  (Rendering|SetVisibility (Variables|Default|GetRangeCollision) (== (Variables|/Game/Blueprints/Game/PC_Game.PC_Game_C|GetSelectedTurret (Variables|Default|GetPC)) self) true))

(fn ConstructionScript
  (bind _range (Variables|Default|GetRange))
  (Components|Sphere|SetSphereRadius (Variables|Default|GetRangeCollision) _range true)
  (Transformation|SetWorldScale3D (Variables|Default|GetRangePlane) (* "1.000000,1.000000,1.000000" (/ _range 5e+01)))
  (Components|Sphere|SetSphereRadius (Variables|Default|GetBlockingCollision) (Variables|Default|GetSize) true))