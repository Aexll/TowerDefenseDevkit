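; Turret placement preview actor that shows a translucent ghost turret and a range plane, tinted green when valid and red when invalid.
; BeginPlay creates dynamic preview and range materials, applies the former to the turret meshes, and caches the PC_Game controller.
; Tick scales the Base mesh from the Size default of the controller's PreviewTurret class.
; SetVisibility toggles the whole component tree, and SetValidity recolors both materials.
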(event Custom|SetVisibility
  (params (NewVisibility :type Boolean))
  (Rendering|SetVisibility (Variables|Default|GetDefaultSceneRoot) NewVisibility true))

(event Custom|SetValidity
  (params (Validity :type Boolean))
  (Rendering|Material|SetVectorParameterValue (Variables|Default|GetDynamicMaterial) "Color" (select Validity "(R=0.000000,G=1.000000,B=0.000000,A=0.100000)" "(R=1.000000,G=0.000000,B=0.000000,A=0.100000)") :!class /Script/Engine.MaterialInstanceDynamic)
  (Rendering|Material|SetVectorParameterValue (Variables|Default|GetDynamicMaterialRange) "Color" (select Validity "(R=0.000000,G=1.000000,B=0.000000,A=0.100000)" "(R=1.000000,G=0.000000,B=0.000000,A=0.100000)") :!class /Script/Engine.MaterialInstanceDynamic))

(event EventBeginPlay
  (bind _returnvalue (Rendering|Material|CreateDynamicMaterialInstance (Variables|Default|GetBase) 0 "/Game/Materials/M_Preview.M_Preview" "None" :!class /Script/Engine.PrimitiveComponent))
  (Variables|Default|SetDynamicMaterial _returnvalue)
  (bind _returnvalue_2 (Rendering|Material|CreateDynamicMaterialInstance (Variables|Default|GetPlane) 0 "/Game/Materials/M_RangeView.M_RangeView" "None" :!class /Script/Engine.PrimitiveComponent))
  (Variables|Default|SetDynamicMaterialRange _returnvalue_2)
  (Rendering|Material|SetMaterial (Variables|Default|GetCannon) 0 (Variables|Default|GetDynamicMaterial))
  (Rendering|Material|SetMaterial (Variables|Default|GetCannon) 1 (Variables|Default|GetDynamicMaterial))
  (Rendering|Material|SetMaterial (Variables|Default|GetCannon) 2 (Variables|Default|GetDynamicMaterial))
  (bind _aspc_game (Utilities|Casting|CastToPC_Game (Game|GetPlayerController 0)))
  (Variables|Default|SetPC _aspc_game))

(event Collision|EventActorBeginOverlap
  (params (OtherActor :type Actor%20Object%20Reference)))

(event EventTick
  (params (DeltaSeconds :type Float%20%28single-precision%29))
  (bind _pc (Variables|Default|GetPC))
  (bind _previewturret (Variables|/Game/Blueprints/Game/PC_Game.PC_Game_C|GetPreviewTurret _pc))
  (if (Utilities|IsValidClass _previewturret)
    (Transformation|SetWorldScale3D (Variables|Default|GetBase) (Math|Conversions|ToVector(Float) (/ (.Size (Utilities|GetClassDefaults _previewturret)) 5e+01)))))

(fn ConstructionScript)