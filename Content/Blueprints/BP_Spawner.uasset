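; BP_Spawner is an enemy spawner that works through a queue of unit names from BeginPlay.
; After each delay it looks up the first ENEMIE entry in the CoreUnits data table and spawns a BP_Enemy at world origin, passing the path, row data and an attribute map.
; It then removes that entry and loops back to the delay, stopping when the queue empties or a row is missing.
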(event EventBeginPlay
  (bind _enemie (Variables|Default|GetENEMIE))
  (Utilities|FlowControl|Delay (Variables|Default|GetDelay) :!label _label)
  (if (Utilities|Array|IsValidIndex _enemie)
    (bind _returnvalue (Utilities|GetDataTableRow "/Game/WavesTools/Datas/CoreUnits.CoreUnits" (Utilities|Array|Get(acopy) _enemie))
      (:then
        (Game|SpawnActorfromClass "/Game/Blueprints/BP_Enemy.BP_Enemy_C" (Math|Transform|MakeTransform "0, 0, 0") "Undefined" 0 (Variables|Default|GetPath) 0.0 _returnvalue (Utilities|Map|MakeMap "NewEnumerator1" true) 0)
        (Utilities|Array|RemoveIndex _enemie)
        (goto _label)))))

(event Collision|EventActorBeginOverlap
  (params (OtherActor :type Actor%20Object%20Reference)))

(event EventTick
  (params (DeltaSeconds :type Float%20%28single-precision%29)))

(fn ConstructionScript)