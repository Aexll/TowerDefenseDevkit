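; First-person player character for a Minecraft-style prototype, with movement, look, jump and block editing.
; Camera line traces drive a per-tick debug box on the targeted grid face, skipped for enemies, and both mouse actions.
; Left click spawns a grid-snapped BP_Block if a box-trace overlap check is clear.
; Right click destroys blocks with a material-matched Niagara effect, or calls Pop on enemies.
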(event EventBeginPlay)

(event Collision|EventActorBeginOverlap
  (params (OtherActor :type Actor%20Object%20Reference)))

(event EventTick
  (params (DeltaSeconds :type Float%20%28single-precision%29))
  (bind _camera (Variables|Default|GetCamera))
  (bind _returnvalue (Math|Vector|GetForwardVector _camera))
  (bind _outhit (Collision|LineTraceByChannel (Transformation|GetWorldLocation _camera) (+ _returnvalue (* _returnvalue 10000)) "TraceTypeQuery1" false 0 "None" true "(R=0.000000,G=0.000000,B=0.000000,A=1.000000)" "(R=0.000000,G=0.000000,B=0.000000,A=1.000000)"))
  (Utilities|Casting|CastToBP_Enemy (.HitActor (Collision|BreakHitResult _outhit))
    (:CastFailed
      (Class|KismetSystemLibrary|BoxTraceMulti (- (Class|KismetMathLibrary|VectorSnappedtoGrid (+ (.Location (Collision|BreakHitResult _outhit)) (* (.Normal (Collision|BreakHitResult _outhit)) 1.0)) 1e+02) (* (.Normal (Collision|BreakHitResult _outhit)) 5e+01)) (- (Class|KismetMathLibrary|VectorSnappedtoGrid (+ (.Location (Collision|BreakHitResult _outhit)) (* (.Normal (Collision|BreakHitResult _outhit)) 1.0)) 1e+02) (* (.Normal (Collision|BreakHitResult _outhit)) 5e+01)) "50.000000,50.000000,0.000000" (Math|Rotator|MakeRotfromZ (.Normal (Collision|BreakHitResult _outhit))) "TraceTypeQuery1" false 0 "ForOneFrame" true "(R=0.000000,G=0.000000,B=0.000000,A=1.000000)" "(R=0.000000,G=0.000000,B=0.000000,A=1.000000)"))))

(event Input|AxisEvents|InputAxisMoveRight
  (params (AxisValue :type Float%20%28single-precision%29))
  (Pawn|Input|AddMovementInput (Math|Vector|GetRightVector (Variables|Collision|GetCapsuleComponent)) AxisValue false))

(event Input|AxisEvents|InputAxisMoveForward
  (params (AxisValue :type Float%20%28single-precision%29))
  (Pawn|Input|AddMovementInput (Math|Vector|GetForwardVector (Variables|Collision|GetCapsuleComponent)) AxisValue false))

(event Input|AxisEvents|InputAxisLookUp
  (params (AxisValue :type Float%20%28single-precision%29))
  (Pawn|Input|AddControllerPitchInput AxisValue))

(event Input|AxisEvents|InputAxisLookRight
  (params (AxisValue :type Float%20%28single-precision%29))
  (Pawn|Input|AddControllerYawInput AxisValue))

(event Input|KeyboardEvents|SpaceBar
  (params (Key :type Key%20Structure))
  (:Pressed
    (Character|Jump)))

(event Input|MouseEvents|RightMouseButton
  (params (Key :type Key%20Structure))
  (bind _camera (Variables|Default|GetCamera))
  (bind _returnvalue (Math|Vector|GetForwardVector _camera))
  (:Pressed
    (bind _outhit (Collision|LineTraceByChannel (Transformation|GetWorldLocation _camera) (+ _returnvalue (* _returnvalue 10000)) "TraceTypeQuery1" false 0 "None"))
    (bind _asbp_block (Utilities|Casting|CastToBP_Block (.HitActor (Collision|BreakHitResult _outhit)))
      (:then
        (bind _returnvalue_2 (Niagara|SpawnSystematLocation "/Game/Particles/P_BlockBreak.P_BlockBreak" (Transformation|GetWorldLocation (Variables|/Game/Blueprints/Old/BP_Block.BP_Block_C|GetBlock _asbp_block))))
        (Class|NiagaraComponent|SetVariableMaterial _returnvalue_2 "Mat" (Rendering|Material|GetMaterial (Variables|/Game/Blueprints/Old/BP_Block.BP_Block_C|GetBlock _asbp_block) 0))
        (Actor|DestroyActor _asbp_block))
      (:CastFailed
        (bind _asbp_enemy (Utilities|Casting|CastToBP_Enemy (.HitActor (Collision|BreakHitResult _outhit))))
        (Default|Pop _asbp_enemy)))))

(event Input|MouseEvents|LeftMouseButton
  (params (Key :type Key%20Structure))
  (bind _camera (Variables|Default|GetCamera))
  (bind _returnvalue (Math|Vector|GetForwardVector _camera))
  (:Pressed
    (bind _outhit (Collision|LineTraceByChannel (Transformation|GetWorldLocation _camera) (+ _returnvalue (* _returnvalue 10000)) "TraceTypeQuery1" false 0 "None"))
    (if (.bBlockingHit (Collision|BreakHitResult _outhit))
      (if (CallFunction|CanPlaceBlock (Class|KismetMathLibrary|VectorSnappedtoGrid (+ (.Location (Collision|BreakHitResult _outhit)) (.Normal (Collision|BreakHitResult _outhit))) 1e+02))
        (Game|SpawnActorfromClass "/Game/Blueprints/Old/BP_Block.BP_Block_C" (Math|Transform|MakeTransform (Class|KismetMathLibrary|VectorSnappedtoGrid (+ (.Location (Collision|BreakHitResult _outhit)) (.Normal (Collision|BreakHitResult _outhit))) 1e+02)) "Undefined" 0 0)))))

(fn ConstructionScript)

(fn CanPlaceBlock
  (params (Location :type Vector))
  (bind _returnvalue (Collision|BoxTraceByChannel Location Location "45.000000,45.000000,45.000000" "0, 0, 0" "TraceTypeQuery1" false 0 "None" false))
  (return (not _returnvalue)))