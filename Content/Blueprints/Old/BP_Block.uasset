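; BP_Block is a block actor whose six faces are textured from the class referenced by its BlockInfo variable.
; When BlockInfo is valid, the construction script creates a dynamic material instance for each of the Block component's six material slots.
; Each instance's Texture parameter takes the matching Forward, Back, Right, Left, Top or Bottom texture from that class's defaults.
; The event graph holds no logic.
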(event EventBeginPlay)

(event Collision|EventActorBeginOverlap
  (params (OtherActor :type Actor%20Object%20Reference)))

(event EventTick
  (params (DeltaSeconds :type Float%20%28single-precision%29)))

(fn ConstructionScript
  (bind _blockinfo (Variables|Default|GetBlockInfo)
    (:then
      (Utilities|FlowControl|Sequence
        (:then_0
          (bind _returnvalue (Rendering|Material|CreateDynamicMaterialInstance (Variables|Default|GetBlock) 0 0 "None" :!class /Script/Engine.PrimitiveComponent))
          (Rendering|Material|SetTextureParameterValue _returnvalue "Texture" (.Forward (Utilities|Struct|BreakS_Texturing (Utilities|GetClassDefaults _blockinfo)))))
        (:then_1
          (bind _returnvalue_2 (Rendering|Material|CreateDynamicMaterialInstance (Variables|Default|GetBlock) 1 0 "None" :!class /Script/Engine.PrimitiveComponent))
          (Rendering|Material|SetTextureParameterValue _returnvalue_2 "Texture" (.Back (Utilities|Struct|BreakS_Texturing (Utilities|GetClassDefaults _blockinfo)))))
        (:then_2
          (bind _returnvalue_3 (Rendering|Material|CreateDynamicMaterialInstance (Variables|Default|GetBlock) 2 0 "None" :!class /Script/Engine.PrimitiveComponent))
          (Rendering|Material|SetTextureParameterValue _returnvalue_3 "Texture" (.Right (Utilities|Struct|BreakS_Texturing (Utilities|GetClassDefaults _blockinfo)))))
        (:then_3
          (bind _returnvalue_4 (Rendering|Material|CreateDynamicMaterialInstance (Variables|Default|GetBlock) 5 0 "None" :!class /Script/Engine.PrimitiveComponent))
          (Rendering|Material|SetTextureParameterValue _returnvalue_4 "Texture" (.Left (Utilities|Struct|BreakS_Texturing (Utilities|GetClassDefaults _blockinfo)))))
        (:then_4
          (bind _returnvalue_5 (Rendering|Material|CreateDynamicMaterialInstance (Variables|Default|GetBlock) 4 0 "None" :!class /Script/Engine.PrimitiveComponent))
          (Rendering|Material|SetTextureParameterValue _returnvalue_5 "Texture" (.Top (Utilities|Struct|BreakS_Texturing (Utilities|GetClassDefaults _blockinfo)))))
        (:then_5
          (bind _returnvalue_6 (Rendering|Material|CreateDynamicMaterialInstance (Variables|Default|GetBlock) 3 0 "None" :!class /Script/Engine.PrimitiveComponent))
          (Rendering|Material|SetTextureParameterValue _returnvalue_6 "Texture" (.Bottom (Utilities|Struct|BreakS_Texturing (Utilities|GetClassDefaults _blockinfo)))))))
    (:else)))