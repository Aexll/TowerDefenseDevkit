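; Path-following block enemy configured from an EnemyInfo row, which sets its texture, size, speed and mesh set, with a Regen mesh variant chosen by attribute.
; Tick advances Time and reads the transform from Path.
; Pop expands the drop table by the given number of layers, spawning children staggered behind on the same path with inherited attributes and immunity tags.
; It then plays a break effect using the block's material and destroys itself.
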(event Custom|Pop
  (params (Pop :type Integer))
  (Utilities|FlowControl|Sequence
    (:then_0
      (bind _newdrops1 (CallFunction|CalculateDrops Pop))
      (for (_array_element _array_index) _newdrops1
        (bind _returnvalue (Utilities|GetDataTableRow "/Game/WavesTools/Datas/CoreUnits.CoreUnits" _array_element)
          (:then
            (bind _returnvalue_2 (Game|SpawnActorfromClass "BP_Enemy_C" (Math|Transform|MakeTransform "0, 0, 0") "Undefined" 0 (Variables|Default|GetPath) (- (Variables|Default|GetTime) (* _array_index 0.03)) _returnvalue (Variables|Default|GetAttributs) 0))
            (bind _result (Utilities|Set|Union (Variables|BP_Enemy_C|GetImuneTags _returnvalue_2) (Variables|Default|GetImuneTags)))
            (Variables|BP_Enemy_C|SetImuneTags _returnvalue_2 _result)))))
    (:then_1
      (bind _returnvalue_3 (Niagara|SpawnSystematLocation "/Game/Particles/P_BlockBreak.P_BlockBreak" (Transformation|GetActorLocation)))
      (Class|NiagaraComponent|SetVariableMaterial _returnvalue_3 "Mat" (Rendering|Material|GetMaterial (Variables|Default|GetCube) 0))
      (Actor|DestroyActor))))

(event EventBeginPlay
  (bind _returnvalue (Rendering|Material|CreateDynamicMaterialInstance (Variables|Default|GetCube) 0 0 "None" :!class /Script/Engine.PrimitiveComponent))
  (Rendering|Material|SetTextureParameterValue _returnvalue "Texture" (.Texture (Utilities|Struct|BreakS_CoreUnit (Variables|Default|GetEnemyInfo))))
  (bind _returnvalue_2 (Utilities|GetDataTableRow "/Game/WavesTools/Datas/ModelsSets.ModelsSets" (Utilities|Struct|BreakS_CoreUnit (Variables|Default|GetEnemyInfo)))
    (:then
      (Components|StaticMesh|SetStaticMesh (Variables|Default|GetCube) (select (.Value (Utilities|Map|Find (Variables|Default|GetAttributs) "Regen")) (.Regen (Utilities|Struct|BreakS_ModelSet _returnvalue_2)) (.Normal (Utilities|Struct|BreakS_ModelSet _returnvalue_2))))
      (Transformation|SetRelativeScale3D (Variables|Default|GetCube) (Math|Conversions|ToVector(Float) (* (.Size (Utilities|Struct|BreakS_CoreUnit (Variables|Default|GetEnemyInfo))) 0.5))))))

(event Collision|EventActorBeginOverlap
  (params (OtherActor :type Actor%20Object%20Reference)))

(event EventTick
  (params (DeltaSeconds :type Float%20%28single-precision%29))
  ;[0 0 0] Comment
  (bind _output_get (Variables|Default|SetTime (+ (Variables|Default|GetTime) (* DeltaSeconds (.Speed (Utilities|Struct|BreakS_CoreUnit (Variables|Default|GetEnemyInfo))) 0.03))))
  (Transformation|SetActorLocation (.WorldLocation (Default|GetLocationatTime (Variables|Default|GetPath) _output_get)) false false)
  (Transformation|SetActorRotation (.WorldRotation (Default|GetLocationatTime (Variables|Default|GetPath) _output_get))))

(fn ConstructionScript)

(fn CalculateDrops
  (params (Recursivity :type Integer))
  (LocalVariables|SetDrops (.Drops (Utilities|Struct|BreakS_CoreUnit (Variables|Default|GetEnemyInfo))))
  (for _index (range 1 Recursivity)
    (Utilities|Array|Clear (LocalVariables|GetNewDrops))
    (for _array_element (LocalVariables|GetDrops)
      (bind _returnvalue (Utilities|GetDataTableRow "/Game/WavesTools/Datas/CoreUnits.CoreUnits" _array_element)
        (:then
          (Utilities|Array|AppendArray (LocalVariables|GetNewDrops) (.Drops (Utilities|Struct|BreakS_CoreUnit _returnvalue))))))
    (LocalVariables|SetDrops (LocalVariables|GetNewDrops)))
  (return (LocalVariables|GetDrops)))